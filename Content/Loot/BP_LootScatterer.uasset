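; Loot spawner that scatters twelve random metal-detecting finds, from junk to coins, across its Plane's area on BeginPlay.
; A fixed-seed random stream, reseeded from itself after each spawn, picks class and position, making the layout repeatable.
; Each item's minimum value is totalled by detector difficulty and printed as a debug summary.
; The exclusive random upper bound of Length-1 means the last class, BP_RareCoin, never spawns.
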(event EventBeginPlay
  (bind _plane (Variables|Default|GetPlane))
  (bind _rarityvalues (Variables|Default|GetRarityValues))
  (bind _returnvalue (Transformation|GetWorldScale _plane))
  (Variables|Default|SetRandom (Math|Random|MakeRandomStream 125))
  (Variables|Default|SetClassArr (Utilities|Array|MakeArray "/Game/Loot/BP_CampingPeg.BP_CampingPeg_C" "/Game/Loot/BP_BottleCap.BP_BottleCap_C" "/Game/Loot/BP_CommonCoin.BP_CommonCoin_C" "/Game/Loot/BP_OldShovel.BP_OldShovel_C" "/Game/Loot/BP_RustyNail.BP_RustyNail_C" "/Game/Loot/BP_RustyMetalDetector.BP_RustyMetalDetector_C" "/Game/Loot/BP_TungstenCube.BP_TungstenCube_C" "/Game/Loot/BP_RareCoin.BP_RareCoin_C"))
  (for _index (range 0 11)
    (bind _returnvalue_2 (Game|SpawnActorfromClass (Utilities|Array|Get(acopy) (Variables|Default|GetClassArr) (Class|KismetMathLibrary|RandomIntegerfromStream (- (Utilities|Array|Length (Variables|Default|GetClassArr)) 1) (Variables|Default|GetRandom))) (Math|Transform|MakeTransform (+ (* (* (Math|Random|RandomUnitVectorfromStream (Variables|Default|GetRandom)) (Math|Vector|MakeVector (.x _returnvalue) (.y _returnvalue) 0.0)) 5e+01) (Transformation|GetWorldLocation (Variables|Default|GetPlane)))) "AlwaysSpawn" 0 0))
    (Math|Random|SetRandomStreamSeed (Variables|Default|GetRandom) (Class|KismetMathLibrary|RandomIntegerfromStream 2147483464 (Variables|Default|GetRandom)))
    (bind _asbp_loot_base (Utilities|Casting|CastToBP_LootBase _returnvalue_2))
    (Utilities|Array|SetArrayElem _rarityvalues (.detectordifficulty (Variables|/Game/Loot/BP_LootBase.BP_LootBase_C|GetLootType _asbp_loot_base)) (+ (Utilities|Array|Get(acopy) _rarityvalues (.detectordifficulty (Variables|/Game/Loot/BP_LootBase.BP_LootBase_C|GetLootType _asbp_loot_base))) (.valuemin (Variables|/Game/Loot/BP_LootBase.BP_LootBase_C|GetLootType _asbp_loot_base)))))
  (for (_array_element _array_index) (Variables|Default|GetRarityValues)
    (Development|PrintString (Utilities|String|Append (Utilities|String|ToString(Integer) _array_index) ": $" (Utilities|String|ToString(Integer) _array_element)) true true "(R=0.098701,G=1.000000,B=0.000000,A=1.000000)" 6e+01)))

(event Collision|EventActorBeginOverlap
  (params (OtherActor :type Actor%20Object%20Reference)))

(event EventTick
  (params (DeltaSeconds :type Float%20%28single-precision%29)))

(fn ConstructionScript)