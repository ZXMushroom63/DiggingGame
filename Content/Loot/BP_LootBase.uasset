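; BP_LootBase is a base loot actor whose appearance and detection tags come from its LootType data.
; The construction script applies the item's mesh and transform and picks a billboard level sprite from its DetectorDifficulty.
; BeginPlay replaces the actor's tags with cumulative "loot" plus index tags from zero through that difficulty, then reapplies the mesh and transform.
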(event EventBeginPlay
  (bind _loottype (Variables|Default|GetLootType))
  (bind _staticmesh (Variables|Default|GetStaticMesh))
  (for _index (range 0 (.detectordifficulty _loottype))
    (Utilities|Array|Add (Variables|Default|GetTagsTemp) (Utilities|String|StringToName (Utilities|String|Append "loot" (Utilities|String|ToString(Integer) _index)))))
  (Variables|Default|SetTags (Variables|Default|GetTagsTemp))
  (Components|StaticMesh|SetStaticMesh _staticmesh (.itemmesh _loottype))
  (Transformation|SetRelativeTransform _staticmesh (.meshtransform _loottype) false false))

(event Collision|EventActorBeginOverlap
  (params (OtherActor :type Actor%20Object%20Reference)))

(event EventTick
  (params (DeltaSeconds :type Float%20%28single-precision%29)))

(fn ConstructionScript
  (bind _loottype (Variables|Default|GetLootType))
  (bind _staticmesh (Variables|Default|GetStaticMesh))
  (Components|StaticMesh|SetStaticMesh _staticmesh (.itemmesh _loottype))
  (Transformation|SetRelativeTransform _staticmesh (.meshtransform _loottype) false false)
  (Rendering|Components|Sprite|SetSprite (Variables|Default|GetBillboard) (Utilities|Array|Get(acopy) (Utilities|Array|MakeArray "/Game/Assets/Loot/T_Level1.T_Level1" "/Game/Assets/Loot/T_Level2.T_Level2" "/Game/Assets/Loot/T_Level3.T_Level3") (.detectordifficulty _loottype))))