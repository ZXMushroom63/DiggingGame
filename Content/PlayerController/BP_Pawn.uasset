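; First-person player pawn for a metal-detecting and digging game, with interaction traces and HUD dialogue.
; Replaces CharacterMovement with velocity-driven capsule physics on Tick, including jumping, friction and air steering.
; The detector tracks the nearest loot for the search level, gating shovel digs that raise and cash it in, advancing Craig's upgrade and radio story via balance.
; Also auto-builds nearby fence segments in FenceMode, forces low graphics settings, and has an L-key loot teleport.
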(event Custom|RadioEvent
  (params (Craig :type BP%20Craig%20Shop%20Object%20Reference))
  (bind _hud (Variables|Default|GetHUD))
  (Variables|Default|SetNoShovelMsg "")
  (Variables|Default|SetShovelEnabled false)
  (Utilities|FlowControl|Delay (Math|Random|RandomFloatinRange 2.0 4.0))
  (Variables|Default|SetNoShovelMsg "Not right now...")
  (Audio|PlaySoundatLocation "/Game/Assets/RadioClip.RadioClip" (Variables|/Game/PlayerController/W_HUD.W_HUD_C|GetTaskLocation _hud) "0, 0, 0" 1.0 1.0 0.0 "/Game/Assets/SA_Attenuate.SA_Attenuate" 0 0)
  (CallFunction|Teletext)
  (Utilities|FlowControl|Delay 3e+01)
  (Variables|Default|SetNoShovelMsg "I should talk to craig first.")
  (Rendering|Components|TextRender|SetText (Variables|/Game/PlayerController/W_HUD.W_HUD_C|GetCurrentObjective _hud) "Talk to Craig About Transmission (Click)")
  (Variables|/Game/PlayerController/W_HUD.W_HUD_C|SetTaskEnabled _hud true)
  (Variables|/Game/Craig/BP_CraigShop.BP_CraigShop_C|SetCraigState Craig "radio_start"))

(event Custom|Teletext
  (bind _hud (Variables|Default|GetHUD))
  (Variables|/Game/PlayerController/W_HUD.W_HUD_C|SetSubtitleMode _hud true)
  (Utilities|FlowControl|Delay 4.0)
  (Default|Splash _hud "\"Your local government, in cooperation with the national weather service, has issued a Civil Danger Warning for Mason County, Illinois.\"" 1.0 true)
  (Utilities|FlowControl|Delay 7.5)
  (Default|Splash _hud "\"Law enforcement are actively searching for a dangerous criminal suspected of multiple homicides.\"" 1.0 true)
  (Utilities|FlowControl|Delay 5.5)
  (Default|Splash _hud "\"The subject was last seen heading to an unknown location within Seamore Forest.\"" 1.0 true)
  (Utilities|FlowControl|Delay 4.5)
  (Default|Splash _hud "\"All residents are advised to secure their homes and shelter in place.\"" 1.0 true)
  (Utilities|FlowControl|Delay 4.5)
  (Default|Splash _hud "\"Do not attempt to approach or apprehend this individual.\"" 1.0 true)
  (Utilities|FlowControl|Delay 4.0)
  (Variables|/Game/PlayerController/W_HUD.W_HUD_C|SetSubtitleMode _hud false))

(event EventBeginPlay
  (bind _self self)
  (bind _output_get (Variables|Default|SetPController (Game|GetPlayerController 0)))
  (Components|Activation|Deactivate (Variables|Character|GetCharacterMovement))
  (CallFunction|LDM)
  (bind _returnvalue (Game|GetCurrentLevelName true))
  (if (Utilities|Enum|Equal(Enum) _returnvalue "BaseLevel")
    (bind _returnvalue_2 (Game|ConstructObjectfromClass "/Game/PlayerController/W_HUD.W_HUD_C" _self))
    (Variables|/Game/PlayerController/W_HUD.W_HUD_C|SetPawn _returnvalue_2 _self)
    (Variables|/Game/PlayerController/W_HUD.W_HUD_C|SetController _returnvalue_2 _output_get)
    (UserInterface|Viewport|AddtoViewport _returnvalue_2 0)
    (Variables|Default|SetHUD _returnvalue_2)))

(event EventTick
  (params (DeltaSeconds :type Float%20%28single-precision%29))
  (CallFunction|GroundCheck)
  (CallFunction|AddGroundFriction DeltaSeconds)
  (CallFunction|JumpandGravity (* DeltaSeconds -5e+02))
  (CallFunction|WASD (Variables|Default|GetPController) DeltaSeconds)
  (CallFunction|TurningReorient DeltaSeconds)
  (CallFunction|AntiBounce DeltaSeconds)
  (CallFunction|PostProcess)
  (CallFunction|AnimateShovel)
  (CallFunction|MetalDetect DeltaSeconds)
  (CallFunction|FenceCode))

(event Input|MouseEvents|MouseX
  (params (AxisValue :type Float%20%28single-precision%29))
  (Pawn|Input|AddControllerYawInput (* AxisValue 1.5)))

(event Input|MouseEvents|MouseY
  (params (AxisValue :type Float%20%28single-precision%29))
  (Pawn|Input|AddControllerPitchInput (* AxisValue -1.5)))

(event Input|KeyboardEvents|SpaceBar
  (params (Key :type Key%20Structure :default "None"))
  (:Pressed
    (Variables|Default|SetIsJumping true))
  (:Released
    (Variables|Default|SetIsJumping false)))

(event Input|KeyboardEvents|L
  (params (Key :type Key%20Structure :default "None"))
  (:Pressed
    (Transformation|SetActorLocation (+ (Transformation|GetActorLocation (Variables|Default|GetMetalDetectTarget)) "0, 0,25.000000") false false)))

(event Input|KeyboardEvents|Enter
  (params (Key :type Key%20Structure :default "None"))
  (:Pressed
    (Default|ConfirmDialogue (Variables|Default|GetHUD))))

(event Input|MouseEvents|LeftMouseButton
  (params (Key :type Key%20Structure :default "None"))
  (bind _hud (Variables|Default|GetHUD))
  (bind _camera (Variables|Default|GetCamera))
  (bind _returnvalue (Transformation|GetWorldLocation _camera))
  (:Pressed
    (if (Variables|Default|GetCutScene)
      (Default|ConfirmDialogue _hud)
      (else
        (Default|ConfirmDialogue _hud)
        (bind _outhit (Collision|LineTraceByChannel _returnvalue (+ _returnvalue (* (Math|Vector|GetForwardVector _camera) 1.1e+02)) "TraceTypeQuery3" false 0 "None"))
        (bind _asi_interactible (Utilities|Casting|CastToI_Interactible (.HitActor (Collision|BreakHitResult _outhit)))
          (:then
            (Default|Interact _asi_interactible self (Variables|Default|GetPController)))
          (:CastFailed
            (CallFunction|DigDown))))))
  (:Released
    (CallFunction|DigUp)))

(event Custom|DigUp
  (Variables|Default|SetTargMetalRot -3.0)
  (Variables|Default|SetTargetProbeDist 0.0))

(event Custom|DigDown
  (bind _digthresh (Variables|Default|GetDigThresh))
  (bind _metaldetecttarget (Variables|Default|GetMetalDetectTarget))
  (bind _targ (Variables|Default|Gettarg))
  (bind _metaldetecttarget_2 (Variables|Default|GetMetalDetectTarget))
  (bind _returnvalue (Transformation|GetWorldLocation _targ))
  (if (not (Variables|Default|GetFenceMode))
    (if (and (Variables|Default|GetShovelEnabled) (not (Variables|Default|GetCutScene)))
      (if (< (.pitch (Transformation|GetWorldRotation (Variables|Default|GetCamera))) -25.0)
        (bind (_outhit _returnvalue_2) (Collision|LineTraceByChannel _returnvalue (+ _returnvalue "0, 0,-20.000000") "TraceTypeQuery1" true 0 "None"))
        (Utilities|IsValid (.HitActor (Collision|BreakHitResult _outhit))
          (:Is%20Valid
            (if (and (Utilities|Array|ContainsItem (Variables|/Script/Engine.Actor|GetTags (.HitActor (Collision|BreakHitResult _outhit))) "gnd") _returnvalue_2)
              (bind _outactors (Actor|GetAllActorswithTag "hole"))
              (if (> (.Distance (Actor|FindNearestActor (.ImpactPoint (Collision|BreakHitResult _outhit)) _outactors)) 36.0)
                (bind _outactors_2 (Actor|GetAllActorswithTag "bush"))
                (if (Math|Boolean|ANDBoolean (Utilities|IsValid _metaldetecttarget) (Variables|Default|GetMetalDetectorClear) (not (Variables|/Game/Loot/BP_LootBase.BP_LootBase_C|GetIsTaken _metaldetecttarget)))
                  (if (> (.Distance (Actor|FindNearestActor (.ImpactPoint (Collision|BreakHitResult _outhit)) _outactors_2)) 6e+01)
                    _
                    (else
                      (Actor|DestroyActor (.ReturnValue (Actor|FindNearestActor (.ImpactPoint (Collision|BreakHitResult _outhit)) _outactors_2)))))
                  (bind _returnvalue_3 (Game|SpawnActorfromClass "/Game/Assets/BP_Hole.BP_Hole_C" (Math|Transform|MakeTransform (.ImpactPoint (Collision|BreakHitResult _outhit)) (Math|Rotator|MakeRotator 0.0 0.0 (Math|Random|RandomFloatinRange 0.0 3.6e+02))) "AlwaysSpawn" 0 0))
                  (Niagara|SpawnSystematLocation "/Game/Assets/NS_Digger.NS_Digger" (.location (Transformation|GetActorTransform _returnvalue_3)) (.rotation (Transformation|GetActorTransform _returnvalue_3)) (.scale (Transformation|GetActorTransform _returnvalue_3)))
                  (Variables|/Game/Loot/BP_LootBase.BP_LootBase_C|SetIsTaken _metaldetecttarget_2 true)
                  (Transformation|SetActorLocation _metaldetecttarget_2 (.Location (Math|Transform|BreakTransform (Math|Transform|MakeTransform (.ImpactPoint (Collision|BreakHitResult _outhit)) (Math|Rotator|MakeRotator 0.0 0.0 (Math|Random|RandomFloatinRange 0.0 3.6e+02))))) false false)
                  (Variables|/Game/Assets/BP_Hole.BP_Hole_C|SetLootItem _returnvalue_3 _metaldetecttarget_2)
                  (Development|SetHiddeninGame (Variables|/Game/Loot/BP_LootBase.BP_LootBase_C|GetStaticMesh _metaldetecttarget_2) false false)
                  (Variables|Default|SetTargMetalRot 1e+01)
                  (Variables|Default|SetTargetProbeDist 45.0))
                (else
                  (Variables|Default|SetTargMetalRot 1e+01)
                  (Variables|Default|SetTargetProbeDist 45.0)
                  (bind _asbp_hole (Utilities|Casting|CastToBP_Hole (.ReturnValue (Actor|FindNearestActor (.ImpactPoint (Collision|BreakHitResult _outhit)) _outactors))))
                  (if (not (>= (Variables|/Game/Assets/BP_Hole.BP_Hole_C|GetDigLevel _asbp_hole) _digthresh))
                    (bind _output_get (Variables|/Game/Assets/BP_Hole.BP_Hole_C|SetDigLevel _asbp_hole (+ (Variables|/Game/Assets/BP_Hole.BP_Hole_C|GetDigLevel _asbp_hole) 1)))
                    (Niagara|SpawnSystematLocation "/Game/Assets/NS_Digger.NS_Digger" (.location (Transformation|GetActorTransform _asbp_hole)) (.rotation (Transformation|GetActorTransform _asbp_hole)) (.scale (Transformation|GetActorTransform _asbp_hole)))
                    (Transformation|SetActorLocation (Variables|/Game/Assets/BP_Hole.BP_Hole_C|GetLootItem _asbp_hole) (Math|Vector|MakeVector (.x (Transformation|GetActorLocation (Variables|/Game/Assets/BP_Hole.BP_Hole_C|GetLootItem _asbp_hole))) (.y (Transformation|GetActorLocation (Variables|/Game/Assets/BP_Hole.BP_Hole_C|GetLootItem _asbp_hole))) (+ (.z (Transformation|GetActorLocation (Variables|/Game/Assets/BP_Hole.BP_Hole_C|GetLootItem _asbp_hole))) (.raiseamount (Variables|/Game/Loot/BP_LootBase.BP_LootBase_C|GetLootType (Variables|/Game/Assets/BP_Hole.BP_Hole_C|GetLootItem _asbp_hole))))) false false)
                    (if (== _output_get _digthresh)
                      (bind _output_get_2 (Variables|Default|Set_tempVal (.valuemin (Variables|/Game/Loot/BP_LootBase.BP_LootBase_C|GetLootType (Variables|/Game/Assets/BP_Hole.BP_Hole_C|GetLootItem _asbp_hole)))))
                      (Default|Splash (Variables|Default|GetHUD) (Utilities|String|Append "You found a " (.name (Variables|/Game/Loot/BP_LootBase.BP_LootBase_C|GetLootType (Variables|/Game/Assets/BP_Hole.BP_Hole_C|GetLootItem _asbp_hole))) " worth $" (Utilities|String|ToString(Integer) (.valuemin (Variables|/Game/Loot/BP_LootBase.BP_LootBase_C|GetLootType (Variables|/Game/Assets/BP_Hole.BP_Hole_C|GetLootItem _asbp_hole)))) "!") 1.5 false)
                      (Variables|Default|SetBalance (+ (Variables|Default|GetBalance) _output_get_2))
                      ;[1 1 1] Comment
                      (CallFunction|BalanceChange)
                      (Actor|DestroyActor (Variables|/Game/Assets/BP_Hole.BP_Hole_C|GetLootItem _asbp_hole))))))))))
      (else
        (Default|Splash (Variables|Default|GetHUD) (Variables|Default|GetNoShovelMsg) 1.0 false)))))

(fn ConstructionScript)

(fn GroundCheck
  (bind _groundcast (Variables|Default|GetGroundCast))
  (bind _returnvalue (Transformation|GetWorldLocation _groundcast))
  (bind _returnvalue_2 (Collision|SphereTraceByChannel _returnvalue (+ _returnvalue (* (Math|Vector|GetForwardVector _groundcast) 15.0)) 2e+01 "TraceTypeQuery1" false 0 "None"))
  (Variables|Default|SetOnGround _returnvalue_2))

(fn AddGroundFriction
  (params (DeltaTime :type Float%20%28single-precision%29))
  (bind _groundfriction (Variables|Default|GetGroundFriction))
  (bind _airresistance (Variables|Default|GetAirResistance))
  (bind _returnvalue (* DeltaTime _groundfriction))
  (bind _returnvalue_2 (* DeltaTime _airresistance))
  (bind _returnvalue_3 (- 1.0 _returnvalue_2))
  (bind _returnvalue_4 (- 1.0 _returnvalue))
  (bind _returnvalue_5 (Math|Float|Clamp(Float) _returnvalue_3))
  (bind _returnvalue_6 (Math|Float|Clamp(Float) _returnvalue_4))
  (if (Variables|Default|GetOnGround)
    (CallFunction|SetVel (* (CallFunction|GetVel) (Math|Vector|MakeVector _returnvalue_6 _returnvalue_6 1.0)))
    (else
      (CallFunction|SetVel (* (CallFunction|GetVel) (Math|Vector|MakeVector _returnvalue_5 _returnvalue_5 1.0))))))

(fn GetVel
  (bind _returnvalue (Physics|GetPhysicsLinearVelocity (Variables|Collision|GetCapsuleComponent) "None"))
  (return _returnvalue))

(fn SetVel
  (params (Vel :type Vector))
  (Physics|SetPhysicsLinearVelocity (Variables|Collision|GetCapsuleComponent) Vel false "None"))

(fn JumpandGravity
  (params (Grav :type Float%20%28single-precision%29))
  (bind _vel (CallFunction|GetVel))
  (if (and (Variables|Default|GetOnGround) (Variables|Default|GetIsJumping))
    (if (< (.z (CallFunction|GetVel)) (/ (Variables|Default|GetJumpPower) 2.0))
      (Variables|Default|SetOnGround false)
      (Variables|Default|SetIsJumping false)
      (CallFunction|SetVel (Math|Vector|MakeVector (.x _vel) (.y _vel) (Variables|Default|GetJumpPower))))
    (elif (not (Variables|Default|GetOnGround))
      (CallFunction|SetVel (+ (CallFunction|GetVel) (Math|Vector|MakeVector 0.0 0.0 Grav))))))

(fn WASD
  (params (PC :type Player%20Controller%20Object%20Reference) (DeltaTime :type Float%20%28single-precision%29))
  (if (Variables|Default|GetCutScene)
    (CallFunction|SetVel "0, 0, 0")
    (else
      (CallFunction|SetVel (+ (CallFunction|GetVel) (Math|Vector|RotateVectorAroundAxis (* (Math|Vector|MakeVector (- (Math|Conversions|ToFloat(Boolean) (Game|Player|IsInputKeyDown PC "W")) (Math|Conversions|ToFloat(Boolean) (Game|Player|IsInputKeyDown PC "S"))) (- (Math|Conversions|ToFloat(Boolean) (Game|Player|IsInputKeyDown PC "D")) (Math|Conversions|ToFloat(Boolean) (Game|Player|IsInputKeyDown PC "A"))) 0.0) (* (Variables|Default|GetSpeed) DeltaTime)) (.yaw (Transformation|GetWorldRotation (Variables|Collision|GetCapsuleComponent))) "0, 0,1.000000"))))))

(fn TurningDeaccel
  (params (DeltaTime :type Float%20%28single-precision%29))
  (bind _vel (CallFunction|GetVel))
  (bind _output_get (LocalVariables|SetnewYaw (.yaw (Transformation|GetWorldRotation (Variables|Collision|GetCapsuleComponent)))))
  (CallFunction|SetVel (Math|Vector|Lerp(Vector) (CallFunction|GetVel) (Math|Vector|MakeVector (* (.x _vel) (Math|Float|Absolute(Float) (Math|Trig|Cos(Degrees) _output_get))) (* (.y _vel) (Math|Float|Absolute(Float) (Math|Trig|Sin(Degrees) _output_get))) (.z _vel)) (Math|Float|Clamp(Float) (* DeltaTime (* (Math|Float|Absolute(Float) (- (Variables|Default|GetPrevYaw) _output_get)) 1.5)))))
  (Variables|Default|SetPrevYaw (LocalVariables|GetnewYaw)))

(fn AntiBounce
  (params (DeltaTime :type Float%20%28single-precision%29))
  (bind _vel (CallFunction|GetVel))
  (bind _returnvalue (Transformation|GetActorLocation))
  (if (and (Variables|Default|GetOnGround) (not (Variables|Default|GetIsJumping)))
    (CallFunction|SetVel (Math|Vector|MakeVector (.x _vel) (.y _vel) 0.0)))
  (if (< (.z _returnvalue) 139.0)
    (Transformation|SetActorLocation (Math|Vector|MakeVector (.x _returnvalue) (.y _returnvalue) 139.0) false true)))

(fn PostProcess
  (Variables|/Script/Engine.CameraComponent|SetPostProcessSettings (Variables|Default|GetCamera) (Utilities|Struct|MakePostProcessSettings "BM_SOG" (+ (/ (Math|Vector|VectorLength (CallFunction|GetVel)) 5e+02) 0.25) 0.0 2.5 -1.0 7.0 0.5 true 0.1 (Utilities|Struct|MakeWeightedBlendables (Utilities|Array|MakeArray (Utilities|Struct|MakeWeightedBlendable 1.0 "/Game/Assets/PS_OptimisedFog.PS_OptimisedFog") (Utilities|Struct|MakeWeightedBlendable 1.0 "/Game/Assets/PS_PostProcess.PS_PostProcess") "")))))

(fn AnimateShovel
  (bind _shovelextender (Variables|Default|GetShovelExtender))
  (bind _hookarm (Variables|Default|GetHookArm))
  (Variables|/Script/Engine.SpringArmComponent|SetTargetArmLength _shovelextender (Math|Float|Lerp (Variables|/Script/Engine.SpringArmComponent|GetTargetArmLength _shovelextender) (Variables|Default|GetTargetProbeDist) 0.75))
  (Transformation|SetRelativeRotation _hookarm (Math|Rotator|MakeRotator 0.0 0.0 (Math|Float|Lerp (.yaw (Variables|/Script/Engine.SceneComponent|GetRelativeRotation _hookarm)) (Variables|Default|GetTargMetalRot) 0.75)) false false))

(fn MetalDetect
  (params (DeltaTime :type Float%20%28single-precision%29))
  (bind _metal_dist (Variables|Default|Getmetal_dist))
  (if (Variables|Default|GetMetalDetectorEnabled)
    (Variables|Default|SetMetalBeepTime (Math|Float|%(Float) (+ (Variables|Default|GetMetalBeepTime) DeltaTime) 2.0))
    (bind _output_get (Variables|Default|SetMetalDetectorTimer (- (Variables|Default|GetMetalDetectorTimer) DeltaTime)))
    (if (< _output_get 0.0)
      (bind _outactors (Actor|GetAllActorswithTag (Utilities|String|StringToName (Utilities|String|Append "loot" (Utilities|String|ToString(Integer) (Variables|Default|GetSearchLevel))))))
      (Utilities|IsValid (.ReturnValue (Actor|FindNearestActor (Transformation|GetWorldLocation (Variables|Default|Gettarg)) _outactors))
        (:Is%20Valid
          (Variables|Default|SetMetalDetectTarget (.AsBP%20Loot%20Base (Utilities|Casting|CastToBP_LootBase (.ReturnValue (Actor|FindNearestActor (Transformation|GetWorldLocation (Variables|Default|Gettarg)) _outactors)))))
          (bind _output_get_2 (LocalVariables|SetFinalDistance (- 10 (Math|Integer|Clamp(Integer) (Math|Float|Round (* (Math|Float|Clamp(Float) (- (Math|Float|Power (Math|Float|Clamp(Float) (* (.Distance (Actor|FindNearestActor (Transformation|GetWorldLocation (Variables|Default|Gettarg)) _outactors)) 0.001)) 0.8) 0.05)) 1e+01)) 0 10))))
          (for _index (range 1 _output_get_2)
            (LocalVariables|SetStr (Utilities|String|Append (LocalVariables|GetStr) "|")))
          (Rendering|Components|TextRender|SetText _metal_dist (Utilities|Text|ToText(String) (LocalVariables|GetStr)))
          (CallFunction|SetMetalDetectorSounds (LocalVariables|GetFinalDistance)))
        (:Is%20Not%20Valid
          (Rendering|Components|TextRender|SetText _metal_dist (Utilities|Text|MakeLiteralText ""))
          (CallFunction|SetMetalDetectorSounds)))
      (Variables|Default|SetMetalDetectorTimer 0.125)
      (Variables|Default|SetMetalDetectorClear (== (- 10 (Math|Integer|Clamp(Integer) (Math|Float|Round (* (Math|Float|Clamp(Float) (- (Math|Float|Power (Math|Float|Clamp(Float) (* (.Distance (Actor|FindNearestActor (Transformation|GetWorldLocation (Variables|Default|Gettarg)) _outactors)) 0.001)) 0.8) 0.05)) 1e+01)) 0 10)) 10)))))

(fn LDM
  (bind _returnvalue (Settings|GetGameUserSettings))
  (Class|GameUserSettings|SetOverallScalabilityLevel _returnvalue)
  (Class|GameUserSettings|SetShadowQuality _returnvalue 3)
  (Class|GameUserSettings|SetPostProcessingQuality _returnvalue)
  (Class|GameUserSettings|SetShadingQuality _returnvalue)
  (Class|GameUserSettings|SetTextureQuality _returnvalue)
  (Class|GameUserSettings|SetAntiAliasingQuality _returnvalue)
  (Class|GameUserSettings|SetResolutionScaleNormalized _returnvalue 0.5)
  (Class|GameUserSettings|SetVisualEffectQuality _returnvalue))

(fn TurningReorient
  (params (DeltaTime :type Float%20%28single-precision%29))
  (if (not (Variables|Default|GetOnGround))
    (bind _output_get (LocalVariables|SetnewYaw (.yaw (Transformation|GetWorldRotation (Variables|Collision|GetCapsuleComponent)))))
    (CallFunction|SetVel (Math|Vector|RotateVectorAroundAxis (CallFunction|GetVel) (* (- (Variables|Default|GetPrevYaw) _output_get) -1.0 (Variables|Default|GetTurningAccuracy)) "0, 0,1.000000"))
    (Variables|Default|SetPrevYaw (LocalVariables|GetnewYaw))))

(fn SetMetalDetectorSounds
  (params (LevelValues :type Integer))
  (bind _snd_metallevela (Variables|Default|GetSND_MetalLevelA))
  (bind _snd_metallevela_2 (Variables|Default|GetSND_MetalLevelA))
  (bind _returnvalue (Audio|Components|Audio|IsPlaying _snd_metallevela))
  (if (> LevelValues 0)
    (if _returnvalue
      _
      (else
        (Audio|Components|Audio|Play _snd_metallevela_2 0.0)))
    (Audio|Components|Audio|SetPitchMultiplier _snd_metallevela_2 (+ (/ (Math|Conversions|ToFloat(Integer) (- LevelValues 1)) 9.0) 1.0))
    (elif _returnvalue
      (Audio|Components|Audio|Stop _snd_metallevela_2))))

(fn SetMetalBeepPlayState
  (params (AudioComponent :type Audio%20Component%20Object%20Reference) (State :type Boolean)))

(fn SetMetalDetector
  (params (New%20State :type Boolean))
  (bind _output_get (Variables|Default|SetMetalDetectorEnabled New%20State))
  (Audio|Components|Audio|SetVolumeMultiplier (Variables|Default|GetSND_MetalLevelA) (CallFunction|Ternary New%20State 0.2 0.0) :!class /Script/Engine.AudioComponent)
  (Development|SetHiddeninGame (Variables|Default|Getmetal_detector) (not _output_get) true))

(fn Ternary
  (params (Condition :type Boolean) (Value :type Float%20%28single-precision%29) (Fallback :type Float%20%28single-precision%29))
  (if Condition
    (return Value)
    (else
      (return Fallback))))

(fn SetShovel
  (params (New%20State :type Boolean))
  (bind _output_get (Variables|Default|SetShovelEnabled New%20State))
  (Development|SetHiddeninGame (Variables|Default|Getshovel) (not _output_get) true))

(fn BalanceChange
  (bind _craigref (Variables|Default|GetCraigRef))
  (bind _hud (Variables|Default|GetHUD))
  (bind _hud_2 (Variables|Default|GetHUD))
  (bind _metaldetector (Variables|/Game/Craig/BP_CraigShop.BP_CraigShop_C|GetMetalDetector _craigref))
  (bind _metaldetector_2 (Variables|/Game/Craig/BP_CraigShop.BP_CraigShop_C|GetMetalDetector _craigref))
  (if (and (Utilities|Enum|Equal(Enum) (Variables|/Game/Craig/BP_CraigShop.BP_CraigShop_C|GetCraigState _craigref) "init_3") (>= (Variables|Default|GetBalance) 10))
    (Variables|/Game/Craig/BP_CraigShop.BP_CraigShop_C|SetCraigState _craigref "upgrade_0")
    (Development|SetHiddeninGame _metaldetector_2 false false)
    (Rendering|Components|TextRender|SetText (Variables|/Game/PlayerController/W_HUD.W_HUD_C|GetCurrentObjective _hud_2) "Upgrade Metal Detector for $10 (Click)")
    (Variables|/Game/PlayerController/W_HUD.W_HUD_C|SetTaskEnabled _hud_2 true)
    (Rendering|Material|SetMaterial _metaldetector_2 2 "/Game/Assets/MetalDetector/CopperCoil.CopperCoil")
    (elif (and (Utilities|Enum|Equal(Enum) (Variables|/Game/Craig/BP_CraigShop.BP_CraigShop_C|GetCraigState _craigref) "upgrade_0-2") (>= (Variables|Default|GetBalance) 16))
      (CallFunction|RadioEvent _craigref)
      (elif (and (Utilities|Enum|Equal(Enum) (Variables|/Game/Craig/BP_CraigShop.BP_CraigShop_C|GetCraigState _craigref) "radio_done") (>= (Variables|Default|GetBalance) 25))
        (Variables|/Game/Craig/BP_CraigShop.BP_CraigShop_C|SetCraigState _craigref "upgrade_1")
        (Development|SetHiddeninGame _metaldetector false false)
        (Rendering|Components|TextRender|SetText (Variables|/Game/PlayerController/W_HUD.W_HUD_C|GetCurrentObjective _hud) "Upgrade Metal Detector for $25 (Click)")
        (Variables|/Game/PlayerController/W_HUD.W_HUD_C|SetTaskEnabled _hud true)
        (Rendering|Material|SetMaterial _metaldetector 2 "/Game/Assets/Loot/Coin/SM_BasicGoldAlloy.SM_BasicGoldAlloy")
        (Rendering|Material|SetMaterial _metaldetector 0 "/Game/Assets/Loot/TungstenCube/M_Tungsten.M_Tungsten")))))

(fn FenceCode
  (bind _hud (Variables|Default|GetHUD))
  (if (Variables|Default|GetFenceMode)
    (LocalVariables|Setpos (Transformation|GetActorLocation))
    (bind _outactors (Actor|GetAllActorsOfClass "/Game/Craig/BP_FenceSegment.BP_FenceSegment_C"))
    (for _array_element _outactors
      (if (and (< (Class|KismetMathLibrary|VectorDistanceSquared (LocalVariables|Getpos) (Transformation|GetActorLocation _array_element)) 4e+04) (not (Variables|/Game/Craig/BP_FenceSegment.BP_FenceSegment_C|GetisBuilt _array_element)))
        (Default|Build _array_element)
        (bind _output_get (Variables|Default|SetFenceCount (- (Variables|Default|GetFenceCount) 1)))
        (if (== _output_get 0)
          (Variables|Default|SetFenceMode false)
          (Variables|Default|SetNoShovelMsg "")
          (Variables|/Game/PlayerController/W_HUD.W_HUD_C|SetSubtitleMode _hud false)
          (Default|BulkVisibilityChange _hud (Utilities|Array|MakeArray (Variables|/Game/PlayerController/W_HUD.W_HUD_C|GetFenceCount _hud) (Variables|/Game/PlayerController/W_HUD.W_HUD_C|GetFenceIcon _hud) (Variables|/Game/PlayerController/W_HUD.W_HUD_C|GetFenceBG _hud)) "Hidden")
          (Variables|Default|SetShovelEnabled true)
          (Variables|Default|SetMetalDetectorEnabled true)
          (Default|Splash (Variables|Default|GetHUD) "All fence built! Resume digging!" 5.0 true))))))