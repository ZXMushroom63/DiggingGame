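; Craig is a knife-wielding enemy that stands facing the player until a random delay ends or the player comes close, then gives chase.
; Tick steps it directly toward BP_Pawn at fixed height, with per-axis clamped speed and no navigation.
; Running is faked by swapping two static meshes on a sine timer, repositioning knives and playing footsteps.
; Any mesh overlap triggers the kill: stab sound, forced look at Craig's head, cutscene flag.
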(event OnComponentBeginOverlap(CraigMesh)
  (params (OverlappedComponent :type Primitive%20Component%20Object%20Reference) (OtherActor :type Actor%20Object%20Reference) (OtherComp :type Primitive%20Component%20Object%20Reference) (OtherBodyIndex :type Integer) (bFromSweep :type Boolean) (SweepResult :type Hit%20Result%20Structure%20%28by%20ref%29))
  (bind _food (Variables|Default|GetFood))
  (Development|PrintString "you are dead")
  (Audio|SpawnSoundatLocation "/Game/Craig/SFX_Stab.SFX_Stab" (Transformation|GetActorLocation) "0, 0, 0" 1.5 1.0 0.0 "/Game/Assets/SA_Attenuate.SA_Attenuate" 0)
  (Variables|Default|SetIsDone true)
  (Variables|Default|SetIsChasing false)
  (Pawn|SetControlRotation (Variables|/Game/PlayerController/BP_Pawn.BP_Pawn_C|GetPController _food) (Math|Rotator|FindLookatRotation (Transformation|GetWorldLocation (Variables|/Game/PlayerController/BP_Pawn.BP_Pawn_C|GetCamera _food)) (Transformation|GetWorldLocation (Variables|Default|GetHeadLoc))))
  (Variables|/Game/PlayerController/BP_Pawn.BP_Pawn_C|SetCutScene (Variables|Default|GetFood) true)
  (Utilities|FlowControl|Delay 1.5)
  (Components|StaticMesh|SetStaticMesh (Variables|Default|GetCraigMesh) "/Game/Craig/Assets/SM_CraigStanding.SM_CraigStanding")
  (Development|SetHiddeninGame (Variables|Default|GetKnifeMesh1) true false)
  (Development|SetHiddeninGame (Variables|Default|GetKnifeMesh2) true false))

(event Custom|Footstep
  (Audio|PlaySoundatLocation (.OutItem (Utilities|Array|Random (Utilities|Array|MakeArray "/Game/PlayerController/SFX_Step2.SFX_Step2" "/Game/PlayerController/SFX_Step2.SFX_Step2"))) (Transformation|GetActorLocation) "0, 0, 0" 0.2 (Math|Random|RandomFloatinRange 0.7 0.9) 0.0 "/Game/Assets/SA_AttenuateX.SA_AttenuateX" 0 0))

(event EventBeginPlay
  (Components|StaticMesh|SetStaticMesh (Variables|Default|GetCraigMesh) "/Game/Craig/Assets/SM_CraigStanding.SM_CraigStanding")
  (Development|PrintString "grr i will attack u")
  (Utilities|FlowControl|Delay 0.01)
  (bind _returnvalue (Actor|GetActorOfClass "/Game/PlayerController/BP_Pawn.BP_Pawn_C"))
  (Variables|Default|SetFood _returnvalue)
  (Utilities|FlowControl|Delay (Math|Random|RandomFloatinRange 1e+01 15.0))
  (Variables|Default|SetIsChasing (not (Variables|Default|GetIsDone))))

(event EventTick
  (params (DeltaSeconds :type Float%20%28single-precision%29))
  (bind _craigmesh (Variables|Default|GetCraigMesh))
  (Utilities|IsValid (Variables|Default|GetFood)
    (:Is%20Valid
      (Variables|Default|SetLookTarget (Transformation|GetWorldLocation (Variables|/Game/PlayerController/BP_Pawn.BP_Pawn_C|GetCamera (Variables|Default|GetFood))))
      (CallFunction|RunningAnimation)
      (CallFunction|ChaseifClose)
      (CallFunction|Movement DeltaSeconds (Variables|Default|GetIsChasing))
      (Transformation|SetWorldRotation _craigmesh (Math|Rotator|MakeRotator 9e+01 0.0 (- (.yaw (Math|Rotator|FindLookatRotation (Transformation|GetWorldLocation _craigmesh) (Variables|Default|GetLookTarget))) 9e+01)) false false))))

(fn ConstructionScript)

(fn RunningAnimation
  (bind _craigmesh (Variables|Default|GetCraigMesh))
  (bind _knifemesh1 (Variables|Default|GetKnifeMesh1))
  (bind _knifemesh2 (Variables|Default|GetKnifeMesh2))
  (bind _staticmesh (Variables|/Script/Engine.StaticMeshComponent|GetStaticMesh _craigmesh))
  (if (Variables|Default|GetIsChasing)
    (if (> (Math|Trig|Sin(Degrees) (* (Utilities|Time|GetRealTimeSeconds) 9e+02)) 0.0)
      (if (!= _staticmesh "/Game/Craig/Assets/SM_CraigRun1.SM_CraigRun1")
        (Components|StaticMesh|SetStaticMesh _craigmesh "/Game/Craig/Assets/SM_CraigRun1.SM_CraigRun1")
        (Transformation|SetRelativeTransform _knifemesh1 (Math|Transform|MakeTransform "-1.187511,-6.722950,3.729584" "-40.000153,89.999374,180.000000" "1,1,1") false false)
        (Transformation|SetRelativeTransform _knifemesh2 (Math|Transform|MakeTransform "0.992189,-5.014539,-3.144591" "-59.999825,89.999023,180.000687" "1,1,1") false false)
        (CallFunction|Footstep :!label _label)
        (Development|SetHiddeninGame (Variables|Default|GetKnifeMesh1) false false)
        (Development|SetHiddeninGame (Variables|Default|GetKnifeMesh2) false false))
      (elif (!= _staticmesh "/Game/Craig/Assets/SM_CraigRun2.SM_CraigRun2")
        (Components|StaticMesh|SetStaticMesh _craigmesh "/Game/Craig/Assets/SM_CraigRun2.SM_CraigRun2")
        (Transformation|SetRelativeTransform _knifemesh1 (Math|Transform|MakeTransform "-1.124973,-5.313463,-2.767374" "-59.999584,89.999046,180.000626" "1,1,1") false false)
        (Transformation|SetRelativeTransform _knifemesh2 (Math|Transform|MakeTransform "0.992189,-5.014539,3.792908" "-59.999825,89.999023,180.000687" "1,1,1") false false)
        (goto _label)))
    (elif (not (Variables|Default|GetIsDone))
      (Development|SetHiddeninGame (Variables|Default|GetKnifeMesh1) true false)
      (Development|SetHiddeninGame (Variables|Default|GetKnifeMesh2) true false))))

(fn ChaseifClose
  (if (< (Math|Vector|Distance(Vector) (Transformation|GetActorLocation (Variables|Default|GetFood)) (Transformation|GetActorLocation)) 7.5e+02)
    (Variables|Default|SetIsChasing (not (Variables|Default|GetIsDone)))))

(fn Movement
  (params (A :type Float%20%28single-precision%29) (Condition :type Boolean))
  (bind _returnvalue (Transformation|GetActorLocation))
  (bind _returnvalue_2 (* A 3.5e+02))
  (bind _food (Variables|Default|GetFood))
  (bind _returnvalue_3 (Transformation|GetActorLocation _food))
  (bind _vel (Default|GetVel _food))
  (bind _returnvalue_4 (* _returnvalue_2 -1.0))
  (bind _returnvalue_5 (* _vel 0.0))
  (bind _returnvalue_6 (+ _returnvalue_3 _returnvalue_5))
  (bind (_x _y) (Math|Vector|BreakVector _returnvalue_6))
  (bind _returnvalue_7 (- (Math|Vector2D|MakeVector2D _x _y) (Math|Vector2D|MakeVector2D (.x _returnvalue) (.y _returnvalue))))
  (bind _returnvalue_8 (Class|KismetMathLibrary|ClampAxes2D _returnvalue_7 _returnvalue_4 _returnvalue_2))
  (if Condition
    (Transformation|SetActorLocation (Math|Vector|MakeVector (+ (.x _returnvalue) (.x _returnvalue_8)) (+ (.y _returnvalue) (.y _returnvalue_8)) 2e+01) false false)
    (Variables|Default|SetLookTarget _returnvalue_6)))