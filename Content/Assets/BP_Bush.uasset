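; BP_Bush is a bush Blueprint that randomizes its look by material.
; Its construction script picks a random entry from MaterialPool and applies it to slot 0 of both Plane and Plane1.
; It also prints a random pool index from a separate evaluation of Random, so that index can differ from the applied material.
; The event graph contains no logic.
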(event EventBeginPlay)

(event EventTick
  (params (DeltaSeconds :type Float%20%28single-precision%29)))

(fn ConstructionScript
  (bind _materialpool (Variables|Default|GetMaterialPool))
  (bind (_outitem _outindex) (Utilities|Array|Random _materialpool))
  (Variables|Default|SetMat _outitem)
  (Development|PrintString (Utilities|String|ToString(Integer) _outindex))
  (Rendering|Material|SetMaterial (Variables|Default|GetPlane) 0 (Variables|Default|GetMat))
  (Rendering|Material|SetMaterial (Variables|Default|GetPlane1) 0 (Variables|Default|GetMat)))